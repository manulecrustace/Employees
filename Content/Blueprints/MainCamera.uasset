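; MainCamera is a player-controlled camera pawn that pans and zooms from input axes.
; MoveForward and MoveRight add movement input along fixed world X and Y, scaled by a movement speed multiplier.
; ZoomIn changes the SpringArm's target arm length by the axis value times a zoom speed multiplier, with no clamping or frame-time scaling.
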(event `InputAxis|MoveForward`
  (params (AxisValue :type "Float (single-precision)"))
  (`self.AddMovementInput` (1.0 0.0 0.0) (* AxisValue (`self.MovementSpeedMultiplier`))))

(event `InputAxis|MoveRight`
  (params (AxisValue :type "Float (single-precision)"))
  (`self.AddMovementInput` (0.0 1.0 0.0) (* AxisValue (`self.MovementSpeedMultiplier`))))

(event `InputAxis|ZoomIn`
  (params (AxisValue :type "Float (single-precision)"))
  (bind _springarm (`self.SpringArm`))
  (set `SpringArmComponent.TargetArmLength` (+ (* AxisValue (`self.ZoomSpeedMultiplier`)) (`SpringArmComponent.TargetArmLength` _springarm)) _springarm))

(fn `UserConstructionScript`)